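; Medium enemy character Blueprint that supplies Idle, Chase and Attack behaviors for a state-driven AI.
; Idle uses the parent's Wander, and Chase moves toward the player only while the StateManager component's current state is ChaseStateAI.
; Attack stops movement and launches stationary bullets from a pooled array along the actor's forward vector, cycling the index.
; A Fire flag alternates shots with a one-second delay to pace firing.
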(event Collision|EventActorBeginOverlap
  (params (OtherActor :type Actor%20Object%20Reference))
  (|CallParentFunction OtherActor) ; This node is disabled and will not be called.\nDrag off pins to build functionality.
)

(event EventTick
  (params (DeltaSeconds :type Float%20%28single-precision%29))
  (|CallParentFunction DeltaSeconds) ; This node is disabled and will not be called.\nDrag off pins to build functionality.
)

(event EventIdle
  ;[1 0.9795 0] Idle Function makes use of parent Wander function
  (CallFunction|Wander))

(event EventChase
  ;[1 0.3688 0] Chase Player Function
  (Variables|Default|SetisWandering false)
  (if (== (Utilities|GetClass (Variables|/Script/UnrealMechanics.StateManager|GetcurrentState (Actor|GetComponentbyClass "/Script/UnrealMechanics.StateManager"))) "/Script/UnrealMechanics.ChaseStateAI")
    (AI|AIMoveTo self "0, 0, 0" (Variables|Default|GetplayerRef) 5.0 true)))

(event EventAttack
  (bind _bp_bulletpool (Variables|Default|GetBP_BulletPool))
  (bind _bulletpool (Variables|/Game/BP_BulletPool.BP_BulletPool_C|GetBulletPool _bp_bulletpool))
  (bind _returnvalue (Utilities|Array|Length _bulletpool))
  ;[1 0.01618 0] Fire Bullets at player but stop moving
  (Class|NavMovementComponent|StopActiveMovement (Variables|Character|GetCharacterMovement))
  (if (and (Variables|Default|GetFire) (> _returnvalue 0))
    (Variables|Default|SetFire false)
    (Variables|Default|SetMaxPool _returnvalue)
    (Utilities|IsValid (Utilities|Array|Get(acopy) _bulletpool (Variables|Default|GetBulletIndex))
      (:Is%20Valid
        (if (Math|Vector|Equal(Vector) (Variables|/Script/Engine.MovementComponent|GetVelocity (Variables|/Game/BP_Bullet.BP_Bullet_C|GetProjectileMovement (Utilities|Array|Get(acopy) _bulletpool (Variables|Default|GetBulletIndex)))) "0, 0, 0" 0.0001)
          (Default|FireBullet (Utilities|Array|Get(acopy) _bulletpool (Variables|Default|GetBulletIndex)) (* (Transformation|GetActorForwardVector) (Variables|/Script/Engine.ProjectileMovementComponent|GetInitialSpeed (Variables|/Game/BP_Bullet.BP_Bullet_C|GetProjectileMovement (Utilities|Array|Get(acopy) _bulletpool (Variables|Default|GetBulletIndex))))))
          (Transformation|DetachFromActor (Utilities|Array|Get(acopy) _bulletpool (Variables|Default|GetBulletIndex)) "KeepWorld" "KeepWorld" "KeepWorld")
          (bind _result (Math|Integer|IncrementInt (Variables|Default|GetBulletIndex))
            (:%20%20
              (bind _output_get (Variables|Default|SetBulletIndex _result))
              (if (== _output_get (Variables|Default|GetMaxPool))
                (Variables|Default|SetBulletIndex 0))))
          (else
            (Development|PrintString "No More Bullets in Pool")))))
    (else
      (Utilities|FlowControl|Delay 1.0)
      (Variables|Default|SetFire true))))

(event EventBeginPlay
  (|CallParentFunction) ; This node is disabled and will not be called.\nDrag off pins to build functionality.
)

(fn ConstructionScript
  (|CallParentFunction))