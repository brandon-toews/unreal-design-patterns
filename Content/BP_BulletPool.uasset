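; BP_BulletPool pre-spawns a set number of BP_Bullet actors for its owner to reuse.
; On BeginPlay it spawns them at the owner's location with mesh collision off, attaches them to the owner, tags each with the owner's first tag and stores them in BulletPool.
; Each bullet's OnBulletDestroyed event is bound to ReturnToPool, which moves it back to the owner and reattaches it.
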(event Custom|ReturnToPool
  (params (Bullet :type BP%20Bullet%20Object%20Reference))
  (bind _returnvalue (Components|GetOwner))
  ;[1 0.8232 0.2929] Generate Pool of Bullets based on the amount set in variable AmountOfBullets
  (Transformation|SetActorLocation Bullet (Transformation|GetActorLocation _returnvalue) false false)
  (Transformation|AttachActorToActor Bullet _returnvalue "None" "KeepWorld" "KeepWorld" "KeepWorld" true))

(event EventBeginPlay
  (bind _returnvalue (Components|GetOwner))
  ;[1 0.8232 0.2929] Generate Pool of Bullets based on the amount set in variable AmountOfBullets
  (for _index (range 0 (Variables|Default|GetAmountOfBullets))
    (bind _returnvalue_2 (Game|SpawnActorfromClass "/Game/BP_Bullet.BP_Bullet_C" (Math|Transform|MakeTransform (Transformation|GetActorLocation (Components|GetOwner)) "0, 0, 0" "1,1,1") "Undefined" 0 0))
    (Collision|SetCollisionEnabled (Variables|/Game/BP_Bullet.BP_Bullet_C|GetBulletMesh _returnvalue_2) "NoCollision")
    (Transformation|AttachActorToActor _returnvalue_2 _returnvalue "None" "KeepWorld" "KeepWorld" "KeepWorld" true)
    (Variables|/Game/BP_Bullet.BP_Bullet_C|SetBulletOwner _returnvalue_2 (Utilities|Array|Get(acopy) (Variables|/Script/Engine.Actor|GetTags _returnvalue)))
    (EventDispatchers|BindEventtoOnBulletDestroyed _returnvalue_2 (delegate Custom|ReturnToPool))
    (Utilities|Array|Add (Variables|Default|GetBulletPool) _returnvalue_2)))