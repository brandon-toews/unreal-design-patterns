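; BP_Spawner is an enemy spawner that produces an enemy about once per second inside its box volume, using a Prototype-style clone pattern.
; BeginPlay spawns and stores one EnemyClass instance, and a Delay on Tick paces SpawnEnemy.
; SpawnEnemy passes a spawn point to that instance and calls Clone, or respawns the instance if invalid.
; FindSpawnSpot line-traces down from random box points, retrying until it hits.
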(event Custom|SpawnEnemy
  ;[1 0.5232 0.2163] Spawn Enemy Function Runs Find Spawn Spot Function, gets enemy character instance and runs its clone function. If there is no enemy character instannce then it spawns one and sets it.
  (bind _spawnpoint (CallFunction|FindSpawnSpot))
  (Utilities|IsValid (Variables|Default|GetSelectedEnemyType)
    (:Is%20Valid
      (Variables|/Game/BP_EnemyCharacterBase.BP_EnemyCharacterBase_C|SetSpawnPoint (Variables|Default|GetSelectedEnemyType) _spawnpoint)
      (Default|Clone (Variables|Default|GetSelectedEnemyType)))
    (:Is%20Not%20Valid
      (bind _returnvalue (Game|SpawnActorfromClass (Variables|Default|GetEnemyClass) (Math|Transform|MakeTransform "0, 0, 0" "0, 0, 0" "1,1,1") "Undefined" 0 0))
      (Variables|Default|SetSelectedEnemyType _returnvalue))))

(event EventBeginPlay
  ;[1 1 1] Begin play spawns an instance of an enemy class and stores it in a pointer
  (bind _returnvalue (Game|SpawnActorfromClass (Variables|Default|GetEnemyClass) (Math|Transform|MakeTransform "0, 0, 0" "0, 0, 0" "1,1,1") "Undefined" 0 0))
  (Variables|Default|SetSelectedEnemyType _returnvalue))

(event Collision|EventActorBeginOverlap
  (params (OtherActor :type Actor%20Object%20Reference)))

(event EventTick
  (params (DeltaSeconds :type Float%20%28single-precision%29))
  ;[1 0.1968 0.8203] Runs SpawnEnemy every sec
  (Utilities|FlowControl|Delay 1.0)
  (CallFunction|SpawnEnemy))

(fn ConstructionScript)

(fn FindSpawnSpot
  (bind _box (Variables|Default|GetBox))
  (bind _returnvalue (Components|Box|GetScaledBoxExtent _box))
  (bind _returnvalue_2 (Transformation|GetWorldLocation _box))
  (bind _returnvalue_3 (Math|Random|RandomPointinBoundingBox _returnvalue_2 _returnvalue))
  ;[0.6446 1 0.552] Find SpawnSpot Function grabs a random location within the box collision box and returns the location
  (bind (_outhit _returnvalue_4) (Collision|LineTraceByChannel _returnvalue_3 (+ _returnvalue_3 "0, 0,-500.000000") "TraceTypeQuery1" true 0 "ForDuration" :!label _label))
  (if _returnvalue_4
    (return (Math|Transform|MakeTransform (.Location (Collision|BreakHitResult _outhit)) "0, 0, 0" "1,1,1"))
    (else
      (goto _label))))