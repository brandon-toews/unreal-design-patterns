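; Spawner actor that creates a random enemy from its class list every second inside its box volume.
; A looping timer calls SpawnEnemy, which gets a transform from FindSpawnSpot, spawns the actor, sets its SpawnPoint, then calls its Clone and Die, so the first instance serves as a template.
; FindSpawnSpot line-traces between random box points, the end offset downward, retrying without limit until it hits a surface.
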(event Custom|SpawnEnemy
  (bind _enemyclass (Variables|Default|GetEnemyClass))
  ;[0.9374 1 0.2172] SpawnEnemy Function randomly selects an enemy class, spawns an actor of that class, then run that actors clone function and finally destroys the inital actor instance
  (bind _spawnpoint (CallFunction|FindSpawnSpot))
  (bind _returnvalue (Game|SpawnActorfromClass (Utilities|Array|Get(acopy) _enemyclass (Math|Random|RandomIntegerinRange 0 (- (Utilities|Array|Length _enemyclass) 1))) _spawnpoint "Undefined" 0 0))
  (Utilities|IsValid _returnvalue
    (:Is%20Valid
      (Variables|/Game/BP_EnemyCharacterBase.BP_EnemyCharacterBase_C|SetSpawnPoint _returnvalue _spawnpoint)
      (Default|Clone _returnvalue)
      (Default|Die _returnvalue))))

(event EventBeginPlay
  ;[1 1 1] BeginPlay function Create timer that runs SpawnEenmy Function every second
  (Utilities|Time|SetTimerbyEvent (delegate Custom|SpawnEnemy) 1.0 true))

(event Collision|EventActorBeginOverlap
  (params (OtherActor :type Actor%20Object%20Reference)))

(fn ConstructionScript)

(fn FindSpawnSpot
  (bind _box (Variables|Default|GetBox))
  (bind _returnvalue (Components|Box|GetScaledBoxExtent _box))
  (bind _returnvalue_2 (Transformation|GetWorldLocation _box))
  (bind _returnvalue_3 (Math|Random|RandomPointinBoundingBox _returnvalue_2 _returnvalue))
  ;[1 0.342 0.141] Find SpawnSpot Function grabs a random location within the box collision box and returns the location
  (bind (_outhit _returnvalue_4) (Collision|LineTraceByChannel _returnvalue_3 (+ _returnvalue_3 "0, 0,-500.000000") "TraceTypeQuery1" true 0 "ForDuration" :!label _label))
  (if _returnvalue_4
    (return (Math|Transform|MakeTransform (.Location (Collision|BreakHitResult _outhit)) "0, 0, 0" "1,1,1"))
    (else
      (goto _label))))