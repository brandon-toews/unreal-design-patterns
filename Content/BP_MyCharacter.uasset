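; Player character Blueprint that overrides the Fire event to shoot bullets from its own BPBulletPool along the actor's forward vector.
; A stationary bullet at the current index is launched at its projectile's initial speed and detached, keeping its world transform.
; The index then advances round-robin through the pool, wrapping at the end.
; If that bullet is still moving, nothing fires and a pool-empty message prints.
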(event EventFire
  (bind _bp_bulletpool (Variables|Default|GetBP_BulletPool))
  (bind _bulletpool (Variables|/Game/BP_BulletPool.BP_BulletPool_C|GetBulletPool _bp_bulletpool))
  (bind _returnvalue (Utilities|Array|Length _bulletpool))
  ;[1 0.3395 0.7573] Override Character Fire Function which grabs bullets from its own bulletpool fires them our of the forward vector of the player.
  (if (> _returnvalue 0)
    (Variables|Default|SetMaxPool _returnvalue)
    (Utilities|IsValid (Utilities|Array|Get(acopy) _bulletpool (Variables|Default|GetBulletIndex))
      (:Is%20Valid
        (if (Math|Vector|Equal(Vector) (Variables|/Script/Engine.MovementComponent|GetVelocity (Variables|/Game/BP_Bullet.BP_Bullet_C|GetProjectileMovement (Utilities|Array|Get(acopy) _bulletpool (Variables|Default|GetBulletIndex)))) "0, 0, 0" 0.0001)
          (Default|FireBullet (Utilities|Array|Get(acopy) _bulletpool (Variables|Default|GetBulletIndex)) (* (Transformation|GetActorForwardVector) (Variables|/Script/Engine.ProjectileMovementComponent|GetInitialSpeed (Variables|/Game/BP_Bullet.BP_Bullet_C|GetProjectileMovement (Utilities|Array|Get(acopy) _bulletpool (Variables|Default|GetBulletIndex))))))
          (Transformation|DetachFromActor (Utilities|Array|Get(acopy) _bulletpool (Variables|Default|GetBulletIndex)) "KeepWorld" "KeepWorld" "KeepWorld")
          (bind _result (Math|Integer|IncrementInt (Variables|Default|GetBulletIndex))
            (:%20%20
              (bind _output_get (Variables|Default|SetBulletIndex _result))
              (if (== _output_get (Variables|Default|GetMaxPool))
                (Variables|Default|SetBulletIndex 0))))
          (else
            (Development|PrintString "No More Bullets in Pool")))))))

(fn ConstructionScript)