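; BP_EnemyCharacterEasy is an enemy character with simple Idle, Chase and Attack behavior events tied to a StateManager component.
; Idle stops active movement and jumps.
; Chase checks that the StateManager's current state is ChaseStateAI, then uses AI Move To to follow the player reference.
; Attack is an empty stub, and BeginPlay, overlap and Tick are disabled placeholders.
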(event EventBeginPlay
  (|CallParentFunction) ; This node is disabled and will not be called.\nDrag off pins to build functionality.
)

(event Collision|EventActorBeginOverlap
  (params (OtherActor :type Actor%20Object%20Reference))
  (|CallParentFunction OtherActor) ; This node is disabled and will not be called.\nDrag off pins to build functionality.
)

(event EventTick
  (params (DeltaSeconds :type Float%20%28single-precision%29))
  (|CallParentFunction DeltaSeconds) ; This node is disabled and will not be called.\nDrag off pins to build functionality.
)

(event EventIdle
  ;[1 0.9795 0] Idle Function just jumps
  (Class|NavMovementComponent|StopActiveMovement (Variables|Character|GetCharacterMovement))
  (Character|Jump))

(event EventChase
  ;[1 0.3688 0] Chase Player Function
  (if (== (Utilities|GetClass (Variables|/Script/UnrealMechanics.StateManager|GetcurrentState (Actor|GetComponentbyClass "/Script/UnrealMechanics.StateManager"))) "/Script/UnrealMechanics.ChaseStateAI")
    (AI|AIMoveTo self "0, 0, 0" (Variables|Default|GetplayerRef) 5.0 true)))

(event EventAttack
  ;[1 0 0.4837] Do Nothing
)

(fn ConstructionScript
  (|CallParentFunction))