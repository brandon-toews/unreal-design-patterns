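; Base enemy character that provides generic behavior events for child classes and dies when hit by a player bullet.
; Idle, Chase and Attack only print placeholders, while Wander uses a flag-gated AI move to random reachable points.
; Clone spawns another enemy of its own class at SpawnPoint.
; Overlapping a player-owned BP_Bullet destroys the enemy and its attached actors, plays explosion effects and destroys the bullet.
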(event Custom|Clone
  ;[1 0.3325 0.588] Generic Clone Function gets class of enemy and spawns that type of enemy
  (Game|SpawnActorfromClass (Utilities|GetClass self) (Variables|Default|GetSpawnPoint) "Undefined" 0 0))

(event Custom|Die
  ;[1 0.04688 0.04688] Die Function destroys the Enemy character and all of the attached bullets
  (Actor|DestroyActor (Actor|GetAttachedActors true))
  (Actor|DestroyActor (Actor|GetAttachedActors true))
  (Actor|DestroyActor (Actor|GetAttachedActors true))
  (Actor|DestroyActor))

(event Custom|Wander
  ;[0.8882 1 0.3708] Generic Wander Function that child classes can use
  (if (not (Variables|Default|GetisWandering))
    (Variables|Default|SetisWandering true)
    (AI|AIMoveTo self (.RandomLocation (AI|Navigation|GetRandomReachablePointinRadius (Transformation|GetActorLocation) 1e+03 0 0)) 0 5.0 false
      (:OnSuccess
        (Utilities|FlowControl|Delay 1.0)
        (Variables|Default|SetisWandering false)))))

(event EventBeginPlay
  ;[1 1 1] Begin by saving a reference to the player and setting isWandering bool to false
  (bind _asmy_character (Utilities|Casting|CastToMyCharacter (Game|GetPlayerCharacter 0)))
  (Variables|Default|SetplayerRef _asmy_character)
  (Variables|Default|SetisWandering false))

(event EventTick
  (params (DeltaSeconds :type Float%20%28single-precision%29)))

(event EventIdle
  ;[0.7801 0.4004 1] Generic Idle Function
  (Development|PrintString "Idle" false true "(R=0.243518,G=1.000000,B=0.348040,A=1.000000)"))

(event EventChase
  ;[0.8094 0.3379 1] Generic Chase Function
  (Development|PrintString "Chase" false true "(R=1.000000,G=0.061979,B=0.530702,A=1.000000)"))

(event EventAttack
  ;[0.8781 0.3511 1] Generic Attack Function
  (Development|PrintString "Attack!!" false true "(R=1.000000,G=0.000000,B=0.026276,A=1.000000)"))

(event Collision|EventActorBeginOverlap
  (params (OtherActor :type Actor%20Object%20Reference))
  (bind _returnvalue (Transformation|GetActorLocation))
  ;[1 1 1] If a bullet collides with enemy check owner of bullet and if the owner is the player's bullet then play explosion animation and sound, run Die Function on enemy and run DestroyBullet function on the bullet
  (if (== (Utilities|GetClass OtherActor) "/Game/BP_Bullet.BP_Bullet_C")
    (bind _asbp_bullet (Utilities|Casting|CastToBP_Bullet OtherActor))
    (if (Utilities|Name|Equal(Name) (Variables|/Game/BP_Bullet.BP_Bullet_C|GetBulletOwner _asbp_bullet) "Player")
      (CallFunction|Die)
      (Effects|SpawnEmitteratLocation "/Game/StarterContent/Particles/P_Explosion.P_Explosion" _returnvalue)
      (Audio|PlaySoundatLocation "/Game/StarterContent/Audio/Explosion_Cue.Explosion_Cue" _returnvalue "0, 0, 0" 1.0 1.0 0.0 0 0 0)
      (Default|DestroyBullet _asbp_bullet))))

(fn ConstructionScript)