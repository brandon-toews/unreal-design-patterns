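; BP_Bullet is a pooled projectile that launches at a given velocity and signals BP_BulletPool through OnBulletDestroyed to be returned.
; FireBullet sets the ProjectileMovement velocity, enables query-only collision after a short delay, then starts a looping timer calling ResetBullet.
; ResetBullet fires the dispatcher and zeroes velocity, while DestroyBullet also disables collision through DeactivateBullet.
; The mesh's overlap event is empty.
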(event OnComponentBeginOverlap(BulletMesh)
  (params (OverlappedComponent :type Primitive%20Component%20Object%20Reference) (OtherActor :type Actor%20Object%20Reference) (OtherComp :type Primitive%20Component%20Object%20Reference) (OtherBodyIndex :type Integer) (bFromSweep :type Boolean) (SweepResult :type Hit%20Result%20Structure%20%28by%20ref%29)))

(event Custom|FireBullet
  (params (Velocity :type Vector))
  ;[1 0.2914 0.3113] Fire Bullet and after bullet has been fired for a certain amount of time it is returned to the pool the OnBulletdestroyed event on the BP_BulletPool
  (Variables|/Script/Engine.MovementComponent|SetVelocity (Variables|Default|GetProjectileMovement) Velocity)
  (Utilities|FlowControl|Delay 0.2)
  (Collision|SetCollisionEnabled (Variables|Default|GetBulletMesh) "QueryOnly")
  (Utilities|Time|SetTimerbyEvent (delegate Custom|ResetBullet) 1e+01 true))

(event Custom|ResetBullet
  ;[1 0.2914 0.3113] Fire Bullet and after bullet has been fired for a certain amount of time it is returned to the pool the OnBulletdestroyed event on the BP_BulletPool
  (Default|CallOnBulletDestroyed self)
  (Variables|/Script/Engine.MovementComponent|SetVelocity (Variables|Default|GetProjectileMovement) "0, 0, 0"))

(event Custom|DeactivateBullet
  ;[1 1 1] DeactivateBullet function sets velocity to zero and turns off collisions
  (Variables|/Script/Engine.MovementComponent|SetVelocity (Variables|Default|GetProjectileMovement) "0, 0, 0")
  (Collision|SetCollisionEnabled (Variables|Default|GetBulletMesh) "NoCollision"))

(event Custom|DestroyBullet
  ;[1 0.3852 0.08067] DestroyBullet function calls DeactivateBullet function and then returns to BulletPool
  (CallFunction|DeactivateBullet)
  (Default|CallOnBulletDestroyed self))

(fn ConstructionScript)